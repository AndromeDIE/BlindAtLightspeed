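; Interactable space shuttle console screen that shows a world-space WBP_ConsoleDisplay for its ConsoleType and lets the player resolve hazards.
; Setup waits one tick for BP_BaseConsole to set the type, then initializes the widget and binds its buttons.
; Player overlap shows an interact prompt, interacting turns the screen on, and leaving turns it off.
; Hazard button clicks are forwarded to the hazard and ship sound systems.
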(event `self.ReceiveBeginPlay`
  ;[0.09896 0.09896 0.09896] Setup
  ;;[1 0.8306 0.3224] For BP_BaseConsole to initialize correct ConsoleType
  (`KismetSystemLibrary.DelayUntilNextTick`)
  (`self.SetupWorldWidget`))

(event `self.ReceiveActorBeginOverlap`
  (params (OtherActor :type "Actor Object Reference"))
  ;[0.09896 0.09896 0.09896] Proximity Handling
  (if (and (`GameplayStatics.ObjectIsA` OtherActor "/Game/Blueprints/Player/BP_PlayerCharacter.BP_PlayerCharacter_C") (not (`SceneComponent.bVisible` (`self.DisplayWidget`))))
    (`self.Event SetInteractPromptVisibility` true)
    (`self.PlayButtonClickSound`)))

(event `self.ReceiveActorEndOverlap`
  (params (OtherActor :type "Actor Object Reference"))
  ;[0.09896 0.09896 0.09896] Proximity Handling
  (if (`GameplayStatics.ObjectIsA` OtherActor "/Game/Blueprints/Player/BP_PlayerCharacter.BP_PlayerCharacter_C")
    (`self.Event DeactivateConsole`)))

(event `Event SetInteractPromptVisibility`
  (params (`Visible?` :type Boolean))
  ;[0.09896 0.09896 0.09896] Interaction-Prompt Visibility
  (`SceneComponent.SetVisibility` (`self.InteractPrompt`) `Visible?` false))

(event `/Game/Blueprints/Interfaces/I_Interactable.OnInteract`
  (params (Interactor :type "Pawn Object Reference"))
  ;[0.09896 0.09896 0.09896] Interaction Handling
  (`self.Event ActivateConsole`))

(event `Event ActivateConsole`
  (bind _displaywidget (`self.DisplayWidget`))
  ;[0.09896 0.09896 0.09896] Show & Hide Console Screen Content on (De-)Activation
  (`self.Event SetInteractPromptVisibility` false)
  (`self.PlayActivateSound`)
  (`/Game/UI/Widgets/ConsoleDisplays/WBP_ConsoleDisplay.Event OnConsoleActivated` (`self.ConsoleDisplayRef`))
  (`PrimitiveComponent.SetCollisionEnabled` _displaywidget "QueryAndPhysics")
  (`SceneComponent.SetVisibility` _displaywidget true false))

(event `Event DeactivateConsole`
  (bind _displaywidget (`self.DisplayWidget`))
  ;[0.09896 0.09896 0.09896] Show & Hide Console Screen Content on (De-)Activation
  (`self.Event SetInteractPromptVisibility` false)
  (`self.PlayDeactivateSound`)
  (`/Game/UI/Widgets/ConsoleDisplays/WBP_ConsoleDisplay.Event OnConsoleDeactivated` (`self.ConsoleDisplayRef`))
  (`PrimitiveComponent.SetCollisionEnabled` _displaywidget "NoCollision")
  (`SceneComponent.SetVisibility` _displaywidget false false))

(event `Event HazardRelatedButtonClicked`
  (params (HazardToResolve :type "/Game/DataTables/Hazards/E_HazardTypes Enum" :default "NewEnumerator0"))
  ;[0.09896 0.09896 0.09896] Console Display Button-Clicked Events
  (`self.PlayButtonClickSound`)
  (`/Game/Blueprints/Hazards/BP_HazardSystem.Event TryResolveHazard` (`/Game/Blueprints/Utils/ResourceLocator.GetHazardSystem`) HazardToResolve)
  (`/Game/Blueprints/SpaceShuttle/SoundSystem/BP_ShipSoundSystem.Event OnHazardRelatedButtonClicked` (`/Game/Blueprints/Utils/ResourceLocator.GetShipSoundSystem`) self HazardToResolve))

(fn `PlayActivateSound`
  (`GameplayStatics.PlaySound2D` (`self.StartupSound`) 1.0 1.0 0.0 null null))

(fn `PlayButtonClickSound`
  (`GameplayStatics.PlaySound2D` (`self.ButtonClickSound`) 1.0 1.0 0.0 null null))

(fn `PlayDeactivateSound`
  (`GameplayStatics.PlaySound2D` (`self.DeactivateSound`) 1.0 1.0 0.0 null null))

(fn `SetupWorldWidget`
  ;[0.1255 0.1255 0.1255] Get Widget Ref
  (bind _aswbp_console_display (cast `/Game/UI/Widgets/ConsoleDisplays/WBP_ConsoleDisplay` (`WidgetComponent.GetWidget` (`self.DisplayWidget`))))
  (bind _output_get (set `self.ConsoleDisplayRef` _aswbp_console_display))
  ;[0.1255 0.1255 0.1255] Initialize Widget
  (`/Game/UI/Widgets/ConsoleDisplays/WBP_ConsoleDisplay.Event Initialize` _output_get (`self.ConsoleType`))
  ;[0.1255 0.1255 0.1255] Bind Widget Button Events
  (add `/Game/UI/Widgets/ConsoleDisplays/WBP_ConsoleDisplay.DeactivateButtonClicked` _output_get (`|CreateDelegate` :!event `Event DeactivateConsole`))
  (add `/Game/UI/Widgets/ConsoleDisplays/WBP_ConsoleDisplay.HazardRelatedButtonClicked` _output_get (`|CreateDelegate` :!event `Event HazardRelatedButtonClicked`))
  (`self.Event DeactivateConsole`))

(fn `UserConstructionScript`)