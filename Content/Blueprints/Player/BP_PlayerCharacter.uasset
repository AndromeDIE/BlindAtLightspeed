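; Player character that handles look-at interaction with world objects and 3D widgets.
; On camera movement, a visibility line trace finds I_Interactable actors and sends look-at start or end calls, skipping the start for the current interaction.
; Interacting calls OnInteract on the looked-at target and plays a success or failure beep.
; A WidgetInteraction component simulates clicks and supplies the trace distance; an event also triggers camera shake.
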(event `self.ReceiveBeginPlay`
  ;[0.09896 0.09896 0.09896] Setup
  (set `self.CheckInteractableLength` (`WidgetInteractionComponent.InteractionDistance` (`self.WidgetInteraction`))))

(event `Event InteractWithNearby`
  ;[0.09896 0.09896 0.09896] LookAt Interaction
  (bind _interactablefound_ (`self.TryInteractWithLookAtInteractable`))
  (if _interactablefound_
    (`GameplayStatics.PlaySound2D` "/Game/Audio/SFX/beep2.beep2" 1.0 1.0 0.0 null null)
    (else
      (`GameplayStatics.PlaySound2D` "/Game/Audio/SFX/beep1.beep1" 1.0 1.0 0.0 null null))))

(event `Event OnCameraMove`
  (bind _firstpersoncamera (`self.FirstPersonCamera`))
  (bind _lookedatinteractable (`self.LookedAtInteractable`))
  (bind _returnvalue (`SceneComponent.K2_GetComponentLocation` _firstpersoncamera))
  (bind _returnvalue_2 (`KismetSystemLibrary.Conv_InterfaceToObject` (`self.CurrentInteraction`)))
  ;[0.09896 0.09896 0.09896] Update LookAt Interactable on Camera- or Player Movement
  (bind _outhit (`KismetSystemLibrary.LineTraceSingle` _returnvalue (+ _returnvalue (* (`SceneComponent.GetForwardVector` _firstpersoncamera) (`self.CheckInteractableLength`))) "TraceTypeQuery1"))
  (bind _asi_interactable (cast `/Game/Blueprints/Interfaces/I_Interactable` (`.HitActor` (`GameplayStatics.BreakHitResult` _outhit)))
    (:`then`
      (bind _output_get (set `self.LookedAtInteractable` _asi_interactable))
      (`/Engine/EditorBlueprintResources/StandardMacros.IsValid` _returnvalue_2
        (:`Is Valid`
          (if (not (== _returnvalue_2 (`KismetSystemLibrary.Conv_InterfaceToObject` _output_get)))
            (`/Game/Blueprints/Interfaces/I_Interactable.OnPlayerLookAt` _output_get :!label _label)))
        (:`Is Not Valid`
          (goto _label))))
    (:`CastFailed`
      (`/Engine/EditorBlueprintResources/StandardMacros.IsValid` (`KismetSystemLibrary.Conv_InterfaceToObject` _lookedatinteractable)
        (:`Is Valid`
          (`/Game/Blueprints/Interfaces/I_Interactable.OnPlayerLookAtEnd` _lookedatinteractable))
        (:`Is Not Valid`
          _))
      (set `self.LookedAtInteractable` null))))

(event `Event OnPressEvent`
  (bind _widgetinteraction (`self.WidgetInteraction`))
  ;[0.09896 0.09896 0.09896] World Widget Interaction
  (`WidgetInteractionComponent.PressPointerKey` _widgetinteraction "LeftMouseButton")
  (`WidgetInteractionComponent.ReleasePointerKey` _widgetinteraction "LeftMouseButton")
  (`KismetSystemLibrary.PrintString` "Player OnPressEvent"))

(event `/Game/Blueprints/Interfaces/I_CameraHolder.CameraShake`
  (`PlayerController.ClientStartCameraShake` :`self` (`GameplayStatics.GetPlayerController` 0) :`Shake` "/Game/Blueprints/Player/BP_CameraShake.BP_CameraShake_C"))

(fn `TryInteractWithLookAtInteractable`
  (returns (`InteractableFound?` :type Boolean))
  (bind _lookedatinteractable (`self.LookedAtInteractable`))
  (`/Engine/EditorBlueprintResources/StandardMacros.IsValid` (`KismetSystemLibrary.Conv_InterfaceToObject` _lookedatinteractable)
    (:`Is Valid`
      (`/Game/Blueprints/Interfaces/I_Interactable.OnInteract` _lookedatinteractable self)
      (set `self.CurrentInteraction` _lookedatinteractable)
      (return true))
    (:`Is Not Valid`
      (set `self.CurrentInteraction` null)
      (return false))))

(fn `UserConstructionScript`)