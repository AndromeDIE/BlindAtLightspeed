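; Ship sound system for the space shuttle that plays hazard resolve sounds when a hazard-related button is clicked.
; The click event searches DT_Hazards for the row matching the hazard type, then plays every sound in that row's ResolveSound map.
; Each map value selects global 2D playback or playback at the triggering actor's location, with 2D as fallback when that actor is invalid.
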(event `Event OnHazardRelatedButtonClicked`
  (params (TriggeringActor :type "Actor Object Reference") (HazardTypeToResolve :type "/Game/DataAssets/Hazards/E_HazardTypes Enum" :default "NewEnumerator0"))
  ;[1 0.6398 0.1534] Get Relevant Data Table Row
  (bind _outrownames (`DataTableFunctionLibrary.GetDataTableRowNames` "/Game/DataAssets/Hazards/DT_Hazards.DT_Hazards"))
  (for _array_element _outrownames
    (bind _returnvalue (`|GetDataTableRow` "/Game/DataAssets/Hazards/DT_Hazards.DT_Hazards" _array_element)
      (:`then`
        (bind ((`Type_4_479AC3C540860D80ADEAC5A67BA39A40` _type) (`MandatoryFailConsequence_28_F12E9FF246B3035C8B6BBC9055367AB1` _mandatoryfailconsequence) (`RandomOptionalFailConsequence_29_165DCEC54B4BC7AFC0EB0F824447DE87` _randomoptionalfailconsequence) (`HazardDisplayName_32_A6A5BB71400FB9A3E1EE688428D43446` _hazarddisplayname) (`ResolveSound_24_32AE27524A67226F20156690639241E5` _resolvesound)) (break `/Game/DataAssets/Hazards/S_Hazard` _returnvalue))
        (if (`|EnumEquality` _type HazardTypeToResolve)
          ;[0.243 0.2978 1] Play All Sounds related to the hazard to resolve
          (bind _keys (`BlueprintMapLibrary.Map_Keys` _resolvesound))
          (for _array_element_2 _keys
            ;;[1 0.4783 0.3379] Decide if sound is played at console location or globally
            (if (or (`BlueprintMapLibrary.Map_Find` _resolvesound _array_element_2) (not (`KismetSystemLibrary.IsValid` TriggeringActor)))
              (`GameplayStatics.PlaySound2D` _array_element_2 1.0 1.0 0.0 null null)
              (else
                (`GameplayStatics.PlaySoundAtLocation` _array_element_2 (`self.K2_GetActorLocation` TriggeringActor) (struct) 1.0 1.0 0.0 "/Game/Audio/ConsoleSoundAttenuation.ConsoleSoundAttenuation" null null null))))
          (break))))))

(fn `UserConstructionScript`)