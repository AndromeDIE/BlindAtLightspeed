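; ResourceLocator is a utility function library that acts as a service locator for game systems owned by BP_GameMode.
; GetHazardSystem and GetShipSoundSystem each cast the current game mode to BP_GameMode and return the matching system reference.
; The lookups depend on that game mode being active, with no fallback when the cast fails.
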(fn `GetHazardSystem`
  (returns (`Out System` :type "/Game/Blueprints/Hazards/BP_HazardSystem Object Reference"))
  (bind _asbp_game_mode (cast `/Game/Blueprints/Game/BP_GameMode` (`GameplayStatics.GetGameMode` (`local.__WorldContext`))))
  (return (`/Game/Blueprints/Game/BP_GameMode.HazardSystem` _asbp_game_mode)))

(fn `GetShipSoundSystem`
  (returns (`Out System` :type "/Game/Blueprints/SpaceShuttle/SoundSystem/BP_ShipSoundSystem Object Reference"))
  (bind _asbp_game_mode (cast `/Game/Blueprints/Game/BP_GameMode` (`GameplayStatics.GetGameMode` (`local.__WorldContext`))))
  (return (`/Game/Blueprints/Game/BP_GameMode.ShipSoundSystem` _asbp_game_mode)))