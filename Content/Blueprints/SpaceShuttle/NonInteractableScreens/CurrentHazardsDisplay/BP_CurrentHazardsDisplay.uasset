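; BP_CurrentHazardsDisplay is a space shuttle screen actor that shows current hazards with their time to resolve.
; BeginPlay caches the WBP_HazardsScreenDisplay from its DisplayWidget component.
; UpdateDisplay converts the incoming hazard list into a map of hazard name to TimeToResolve and passes it to the widget.
; Duplicate hazard names get an incrementing number appended so every map key stays unique.
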(event `self.ReceiveBeginPlay`
  (bind _aswbp_hazards_screen_display (cast `/Game/UI/Widgets/ConsoleDisplays/WBP_HazardsScreenDisplay` (`WidgetComponent.GetWidget` (`self.DisplayWidget`))))
  (set `self.HazardDisplayRef` _aswbp_hazards_screen_display))

(event `Event UpdateDisplay`
  (params (HazardList :type "Array of /Game/Blueprints/Hazards/BP_HazardObject Object Reference"))
  (bind _displaymap (`self.GetMapForDisplay` HazardList))
  (`/Game/UI/Widgets/ConsoleDisplays/WBP_HazardsScreenDisplay.Event UpdateDisplay` (`self.HazardDisplayRef`) _displaymap))

(fn `GetMapForDisplay`
  (params (HazardList :type "Array of /Game/Blueprints/Hazards/BP_HazardObject Object Reference"))
  (returns (DisplayMap :type "Map of String to Float (double-precision)"))
  (locals (RetVal :type "Map of String to Float (double-precision)") (KeyString :type String) (NewIndex :type Integer :default 1))
  (for _array_element HazardList
    (bind _hazardname (`/Game/Blueprints/Utils/HazardTypeNameGetter.GetHazardName` (`/Game/Blueprints/Hazards/BP_HazardObject.HazardType` _array_element)))
    (set `local.KeyString` _hazardname)
    (while (`.ReturnValue` (`BlueprintMapLibrary.Map_Find` (`local.RetVal`) (`local.KeyString`)))
      (bind _output_get (set `local.KeyString` _hazardname))
      (set `local.KeyString` (`KismetStringLibrary.Concat_StrStr` _output_get (`KismetStringLibrary.Conv_IntToString` (`local.NewIndex`))))
      (`/Engine/EditorBlueprintResources/StandardMacros.IncrementInt` (`local.NewIndex`)))
    (`BlueprintMapLibrary.Map_Add` (`local.RetVal`) (`local.KeyString`) (`/Game/Blueprints/Hazards/BP_HazardObject.TimeToResolve` _array_element)))
  (return (`local.RetVal`)))

(fn `UserConstructionScript`)