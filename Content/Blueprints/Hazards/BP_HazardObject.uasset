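; BP_HazardObject represents a timed hazard that penalizes the player if it is not resolved in time.
; OnCreation copies type, consequences and time limit from the supplied hazard data and starts a one-shot timer, while Resolve flags it resolved.
; On unresolved timeout, it calls ResolveFailed with a formatted message for every mandatory consequence, then random optional picks, repeats possible, to fill ConsequenceAmount.
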(event `Event Resolve`
  (set `self.IsResolved?` true))

(event `Event OnCreation`
  (params (`New Hazard` :type "/Game/DataAssets/Hazards/S_Hazard Structure"))
  (bind ((`Type_4_479AC3C540860D80ADEAC5A67BA39A40` _type) (`MandatoryFailConsequence_28_F12E9FF246B3035C8B6BBC9055367AB1` _mandatoryfailconsequence) (`RandomOptionalFailConsequence_29_165DCEC54B4BC7AFC0EB0F824447DE87` _randomoptionalfailconsequence) (`ConsequenceAmount_9_992533D24B86F2A3B10C97873BCFCAA2` _consequenceamount) (`TimeToResolve_12_7238684243192D2DE3AF5F93753DF317` _timetoresolve)) (break `/Game/DataAssets/Hazards/S_Hazard` `New Hazard`))
  (set `self.HazardType` _type)
  (set `self.MandatoryFailConsequence` _mandatoryfailconsequence)
  (set `self.OptionalRandomConsequenceOfFailure` _randomoptionalfailconsequence)
  (set `self.ConsequenceAmount` _consequenceamount)
  (bind _output_get (set `self.TimeToResolve` _timetoresolve))
  (`KismetSystemLibrary.K2_SetTimerDelegate` (delegate `Event OnResolveTimeExceeded`) _output_get)
  (`KismetSystemLibrary.PrintString` null "New Hazard Created!"))

(event `Event OnResolveTimeExceeded`
  (if (not (`self.IsResolved?`))
    (`|ExecutionSequence`
      (:`then_0`
        ;[1 1 1] Mandatory Consequences
        (for _array_element (`self.MandatoryFailConsequence`)
          (`self.ResolveFailed` (`self.GetConsequenceFailMessage` _array_element) _array_element self)))
      (:`then_1`
        ;[1 1 1] Optional Random Consequences
        (for _ (range (+ (- (`self.ConsequenceAmount`) 1 (`KismetArrayLibrary.Array_Length` (`self.MandatoryFailConsequence`))) 1))
          (bind (_fail_message _consequence) (`self.GetRandomConsequenceFromSelection`))
          (`self.ResolveFailed` _fail_message _consequence self))))))

(fn `GetConsequenceFailMessage`
  (params (Enumerator :type "/Game/DataAssets/Hazards/E_FailureConsequence Enum" :default "NewEnumerator1"))
  (returns (Result :type Text))
  (return (`|FormatText` "Hazard of type {HazardType} was not resolved. Player suffers {Consequence}!" (`|GetEnumeratorNameAsString` (`self.HazardType`)) (`|GetEnumeratorNameAsString` Enumerator))))

(fn `GetRandomConsequenceFromSelection`
  (returns (`Fail Message` :type Text) (Consequence :type "/Game/DataAssets/Hazards/E_FailureConsequence Enum"))
  (locals (FailConsequence :type "/Game/DataAssets/Hazards/E_FailureConsequence Enum"))
  (bind _optionalrandomconsequenceoffailure (`self.OptionalRandomConsequenceOfFailure`))
  (bind _output_get (set `local.FailConsequence` (`|GetArrayItem` _optionalrandomconsequenceoffailure (`KismetMathLibrary.RandomInteger` (- (`KismetArrayLibrary.Array_Length` _optionalrandomconsequenceoffailure) 1)))))
  (return (`self.GetConsequenceFailMessage` _output_get) _output_get))