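; BP_GameActionManager links level buttons to game actions such as winning or losing the game.
; On BeginPlay it binds to the pressed event of every BP_Button in the level.
; An action class is instantiated, bound to and executed through CreateAndRunGameAction.
; Action types are handled in HandleGameActionExecute, which calls the game mode's win or lose message, or prints a notice for an empty action.
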(event `self.ReceiveBeginPlay`
  (bind _outactors (`GameplayStatics.GetAllActorsOfClass` "/Game/Blueprints/SpaceShuttle/Interactables/Buttons/BP_Button.BP_Button_C"))
  (for _array_element _outactors
    (add `/Game/Blueprints/SpaceShuttle/Interactables/Buttons/BP_Button.Pressed` _array_element (`|CreateDelegate` :!event `Event CreateAndRunGameAction`))
    (`KismetSystemLibrary.PrintString` "Button added")))

(event `Event CreateAndRunGameAction`
  (params (ActionToTrigger :type "/Game/Blueprints/Game/GameActions/BP_BaseGameAction Class Reference"))
  (bind _returnvalue (`|GenericCreateObject` ActionToTrigger))
  (add `/Game/Blueprints/Game/GameActions/BP_BaseGameAction.Execute` _returnvalue (`|CreateDelegate` :!event `Event HandleGameActionExecute`))
  (`/Game/Blueprints/Game/GameActions/BP_BaseGameAction.Event Execute` _returnvalue null))

(event `Event HandleGameActionExecute`
  (params (GameActionType :type "/Game/Blueprints/Game/GameActions/E_GameActionTypes Enum" :default "NewEnumerator2"))
  (switch `/Game/Blueprints/Game/GameActions/E_GameActionTypes` GameActionType
    (:`NewEnumerator2`
      (`KismetSystemLibrary.PrintString` "Empty game action triggered!"))
    (:`NewEnumerator0`
      (message `/Game/Blueprints/Game/BPI_Game.WinGame` (`GameplayStatics.GetGameMode`)))
    (:`NewEnumerator1`
      (message `/Game/Blueprints/Game/BPI_Game.LoseGame` (`GameplayStatics.GetGameMode`)))))

(fn `UserConstructionScript`)