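; Game mode for a shuttle hazard game that runs the hazard loop, score and game over flow.
; Creates the hazard system, ship sound system and score widget, then each Tick updates hazards and their displays.
; Resolved hazards add score, while failed ones trigger a new hazard, game over, console disabling or camera shake, the latter two via interface messages.
; Game over pauses play and opens a Tick gate for a countdown that reloads Main.
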(event `self.ReceiveBeginPlay`
  ;[0.02336 0.05729 0.02576] Setup
  ;;[1 0.2745 0] Hazard System Setup
  (bind _returnvalue (`|GenericCreateObject` "/Game/Blueprints/Hazards/BP_HazardSystem.BP_HazardSystem_C"))
  (bind _output_get (set `self.HazardSystem` _returnvalue))
  (add `/Game/Blueprints/Hazards/BP_HazardSystem.NewHazardCreated` _output_get (delegate `Event OnNewHazardCreated`))
  (`/Game/Blueprints/Hazards/BP_HazardSystem.Event OnCreate` _output_get)
  ;;[0.04911 0.2517 1] Ship Sound System Setup
  (bind _returnvalue_2 (`|SpawnActorFromClass` "/Game/Blueprints/SpaceShuttle/SoundSystem/BP_ShipSoundSystem.BP_ShipSoundSystem_C" (`KismetMathLibrary.MakeTransform` (0.0 0.0 0.0)) "Undefined" "MultiplyWithRoot" null null))
  (set `self.ShipSoundSystem` _returnvalue_2)
  ;;[1 0.1036 0.1335] Shuttle Hazard Display Setup
  (bind _outactors (`GameplayStatics.GetAllActorsOfClass` "/Game/Blueprints/SpaceShuttle/NonInteractableScreens/CurrentHazardsDisplay/BP_CurrentHazardsDisplay.BP_CurrentHazardsDisplay_C"))
  (set `self.HazardDisplays` _outactors)
  ;;[0.06368 0.5003 0.5104] Score Setup
  (bind _returnvalue_3 (`|CreateWidget` "/Game/UI/Widgets/Overlays/WBP_Score.WBP_Score_C"))
  (bind _output_get_2 (set `self.ScoreDisplay` _returnvalue_3))
  (`UserWidget.AddToViewport` _output_get_2 0))

(event `Event OnNewHazardCreated`
  (params (CreatedHazard :type "/Game/Blueprints/Hazards/BP_HazardObject Object Reference") (WarnMessage :type Text))
  ;[0.02336 0.05729 0.02576] Setup
  ;;[1 0.2745 0] Hazard System Setup
  (add `/Game/Blueprints/Hazards/BP_HazardObject.ResolveFailed` CreatedHazard (delegate `Event OnHazardResolveFailed`))
  (add `/Game/Blueprints/Hazards/BP_HazardObject.Resolve` CreatedHazard (`|CreateDelegate` :!event `Event OnHazardResolve`))
  (`KismetSystemLibrary.PrintText` WarnMessage true true (struct :`R` 1.0 :`G` 0.659657 :`A` 1.0)))

(event `Event OnHazardResolveFailed`
  (params (`Fail Message` :type Text) (Consequence :type "/Game/DataAssets/Hazards/E_FailureConsequence Enum" :default "NewEnumerator1") (UnresolvedHazard :type "/Game/Blueprints/Hazards/BP_HazardObject Object Reference"))
  ;[0.02336 0.05729 0.02576] Setup
  ;;[1 0.2745 0] Hazard System Setup
  (`KismetSystemLibrary.PrintText` `Fail Message` true true (struct :`R` 1.0 :`B` 0.028928 :`A` 1.0))
  (`self.HandleFailConsequence` Consequence))

(event `Event OnHazardResolve`
  (params (ResolvedHazard :type "/Game/Blueprints/Hazards/BP_HazardObject Object Reference"))
  ;[0.02336 0.05729 0.02576] Setup
  ;;[1 0.2745 0] Hazard System Setup
  (bind _result (`/Engine/EditorBlueprintResources/StandardMacros.IncrementInt` (`self.CurrentScore`))
    (:`  `
      (`/Game/UI/Widgets/Overlays/WBP_Score.Event UpdateScore` (`self.ScoreDisplay`) _result))))

(event `Event GameOver`
  ;[0.3698 0.01713 0] Game Over
  (`GameplayStatics.SetGamePaused` true)
  (bind _returnvalue (`|CreateWidget` "/Game/UI/Widgets/Overlays/WBP_GameOverScreen.WBP_GameOverScreen_C"))
  (bind _output_get (set `self.GameOverWidget` _returnvalue))
  (`UserWidget.AddToViewport` _output_get 0)
  (set `self.GameOverTimeLeft` (`self.GameOverTime`))
  (`self.Event OpenGameOverGate`)
  (`/Game/Blueprints/Hazards/BP_HazardSystem.Event OnGameOver` (`self.HazardSystem`)))

(event `Event OpenGameOverGate`
  ;[0.07812 0.07812 0.07812] Tick
  (goto _label :!via `Open`))

(event `self.ReceiveTick`
  (params (DeltaSeconds :type "Float (single-precision)"))
  ;[0.07812 0.07812 0.07812] Tick
  (`|ExecutionSequence`
    (:`then_0`
      ;;[0.651 0.04747 0.04747] Game Over Countdown
      (`/Engine/EditorBlueprintResources/StandardMacros.Gate` true :!label _label
        (:`Exit`
          (`self.HandleGameOverTimeLeft` DeltaSeconds))))
    (:`then_1`
      ;;[1 0.3513 0] Hazard Display Update
      (for _array_element (`self.HazardDisplays`)
        (`/Game/Blueprints/SpaceShuttle/NonInteractableScreens/CurrentHazardsDisplay/BP_CurrentHazardsDisplay.Event UpdateDisplay` _array_element (`/Game/Blueprints/Hazards/BP_HazardSystem.ActiveHazards` (`self.HazardSystem`)))))
    (:`then_2`
      ;;[1 0.927 0] Hazard Tick
      (`/Game/Blueprints/Hazards/BP_HazardSystem.Event Tick` (`self.HazardSystem`) DeltaSeconds))))

(event `Event OnDisableConsequence`
  (bind _outactors (`GameplayStatics.GetAllActorsWithInterface` "/Game/Blueprints/Interfaces/I_Deactivatable.I_Deactivatable_C"))
  (for _array_element _outactors
    (message `/Game/Blueprints/Interfaces/I_Deactivatable.Deactivate` _array_element 2.5)))

(fn `HandleFailConsequence`
  (params (Consequence :type "/Game/DataAssets/Hazards/E_FailureConsequence Enum" :default "NewEnumerator1"))
  (switch `/Game/DataAssets/Hazards/E_FailureConsequence` Consequence
    (:`NewEnumerator2`
      (`/Game/Blueprints/Hazards/BP_HazardSystem.Event CreateRandomHazard` (`self.HazardSystem`)))
    (:`NewEnumerator0`
      (`self.Event GameOver`))
    (:`NewEnumerator3`
      (`self.Event OnDisableConsequence`))
    (:`NewEnumerator7`
      (`self.StartCameraShake`))))

(fn `HandleGameOverTimeLeft`
  (params (DeltaTime :type "Float (double-precision)"))
  (bind _output_get (set `self.GameOverTimeLeft` (- (`self.GameOverTimeLeft`) DeltaTime)))
  (`self.UpdateWidgetTimer` _output_get)
  (if (< _output_get 0.0)
    (`GameplayStatics.SetGamePaused` false)
    (`GameplayStatics.OpenLevel` "Main")))

(fn `StartCameraShake`
  (bind _outactors (`GameplayStatics.GetAllActorsWithInterface` "/Game/Blueprints/Interfaces/I_CameraHolder.I_CameraHolder_C"))
  (for _array_element _outactors
    (message `/Game/Blueprints/Interfaces/I_CameraHolder.CameraShake` _array_element)))

(fn `UpdateWidgetTimer`
  (params (Value :type "Float (double-precision)"))
  (set `/Game/UI/Widgets/Overlays/WBP_GameOverScreen.TimeLeftText` (`KismetTextLibrary.Conv_DoubleToText` Value "HalfToEven") (`self.GameOverWidget`)))

(fn `UserConstructionScript`)