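; Base actor for space shuttle interactables that highlights itself while the player looks at it.
; OnPlayerLookat applies FrameMaterial as an overlay material to every static mesh component under DefaultSceneRoot, including nested children.
; OnPlayerLookatEnd walks the same components and clears the overlay.
; The file holds no look detection or interaction logic, and BeginPlay, Tick and overlap events are unused.
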(event `/Game/Blueprints/Interfaces/I_Interactable.OnPlayerLookAt`
  (for _array_element (`SceneComponent.GetChildrenComponents` (`self.DefaultSceneRoot`) true)
    (bind _asstatic_mesh_component (cast `StaticMeshComponent` _array_element))
    (`MeshComponent.SetOverlayMaterial` _asstatic_mesh_component "/Engine/VREditor/UI/FrameMaterial.FrameMaterial")))

(event `/Game/Blueprints/Interfaces/I_Interactable.OnPlayerLookAtEnd`
  (for _array_element (`SceneComponent.GetChildrenComponents` (`self.DefaultSceneRoot`) true)
    (bind _asstatic_mesh_component (cast `StaticMeshComponent` _array_element))
    (`MeshComponent.SetOverlayMaterial` _asstatic_mesh_component null)))

(fn `UserConstructionScript`)