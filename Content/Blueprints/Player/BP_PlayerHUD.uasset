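; BP_PlayerHUD is the player HUD, showing a crosshair and an interaction prompt.
; On BeginPlay it adds the crosshair widget, then binds to the player character's looking-at-interactable, look-end and interacted events.
; Separate show and remove events manage a single tracked prompt widget, creating a fresh one on each show after removing any existing one.
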(event `self.ReceiveBeginPlay`
  (bind _returnvalue (`GameplayStatics.GetPlayerController` 0))
  (bind _returnvalue_2 (`|CreateWidget` "/Game/UI/Widgets/PlayerHUD/WBP_CrossHair.WBP_CrossHair_C" _returnvalue))
  (bind _output_get (set `self.CrosshairRef` _returnvalue_2))
  (`UserWidget.AddToViewport` _output_get 0)
  (bind _asbp_player_character (cast `/Game/Blueprints/Player/BP_PlayerCharacter` (`Controller.K2_GetPawn` _returnvalue)))
  (add `/Game/Blueprints/Player/BP_PlayerCharacter.LookingAtInteractable` _asbp_player_character (`|CreateDelegate` :!event `Event ShowInteractionPrompt`))
  (add `/Game/Blueprints/Player/BP_PlayerCharacter.LookingAtInteractableEnd` _asbp_player_character (`|CreateDelegate` :!event `Event RemoveInteractionPrompt`))
  (add `/Game/Blueprints/Player/BP_PlayerCharacter.Interacted` _asbp_player_character (`|CreateDelegate` :!event `Event RemoveInteractionPrompt`)))

(event `Event ShowInteractionPrompt`
  (bind _currentinteractprompt (`self.CurrentInteractPrompt`)
    (:`then`
      (`Widget.RemoveFromParent` _currentinteractprompt))
    (:`else`
      _))
  (bind _returnvalue (`|CreateWidget` "/Game/UI/Widgets/Overlays/WBP_InteractionPrompt.WBP_InteractionPrompt_C"))
  (bind _output_get (set `self.CurrentInteractPrompt` _returnvalue))
  (`UserWidget.AddToViewport` _output_get 0))

(event `Event RemoveInteractionPrompt`
  (bind _currentinteractprompt (`self.CurrentInteractPrompt`)
    (:`then`
      (`Widget.RemoveFromParent` _currentinteractprompt)
      (set `self.CurrentInteractPrompt` null))
    (:`else`)))

(fn `UserConstructionScript`)